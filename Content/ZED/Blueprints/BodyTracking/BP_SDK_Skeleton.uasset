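; Debug-style skeleton actor that draws a ZED body-tracking pose with spheres for joints and cylinders for bones.
; BeginPlay hides its skeletal mesh, then spawns and attaches one randomly colored sphere and cylinder per camera keypoint, optionally sharing one color.
; Move functions place these at supplied keypoints with a fixed Y offset, choosing the 34, 38 or 70-body bone table by array length.
; Show functions toggle visibility and collision.
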(event EventBeginPlay
  (bind _skeletalmesh (Variables|Default|GetSkeletalMesh))
  (Utilities|FlowControl|Sequence
    (:then_0
      (Collision|SetCollisionEnabled _skeletalmesh "NoCollision")
      (Rendering|SetVisibility _skeletalmesh false true))
    (:then_1
      ;[1 1 1] Fill array of node nodes actors (spheres)
      (for _index (range 0 (- (Class|SlCameraProxy|GetNumberOfKeypoints (Class|SlFunctionLibrary|GetCameraProxy)) 1))
        (bind _returnvalue (Game|SpawnActorfromClass "/Game/ZED/Blueprints/BodyTracking/BP_CustomSphere.BP_CustomSphere_C" (Math|Transform|MakeTransform (Transformation|GetWorldLocation (Variables|Default|GetRoot)) "0, 0, 0" "0.600000,0.600000,0.600000") "AlwaysSpawn" 0 0))
        (Rendering|Material|SetVectorParameterValueonMaterials (Variables|/Script/Engine.StaticMeshActor|GetStaticMeshComponent _returnvalue) "MaterialColor" (CallFunction|GiveColorDependingonIndex _index))
        (Transformation|AttachActorToActor _returnvalue self "None" "KeepRelative" "KeepRelative" "KeepRelative" true)
        (Utilities|Array|Add (Variables|Default|GetNodes) _returnvalue)))
    (:then_2
      ;[1 1 1] Fill array of bones actors (cylinders)
      (for _index_2 (range 0 (- (Class|SlCameraProxy|GetNumberOfKeypoints (Class|SlFunctionLibrary|GetCameraProxy)) 1))
        (bind _returnvalue_2 (Game|SpawnActorfromClass "/Game/ZED/Blueprints/BodyTracking/BP_CustomCylinder.BP_CustomCylinder_C" (Math|Transform|MakeTransform (Transformation|GetWorldLocation (Variables|Default|GetRoot)) "0, 0, 0" "0.100000,0.100000,0.100000") "AlwaysSpawn" self 0))
        (Rendering|Material|SetVectorParameterValueonMaterials (Variables|/Script/Engine.StaticMeshActor|GetStaticMeshComponent _returnvalue_2) "MaterialColor" (CallFunction|GiveColorDependingonIndex _index_2))
        (Transformation|AttachActorToActor _returnvalue_2 self "None" "KeepRelative" "KeepRelative" "KeepRelative" true)
        (Utilities|Array|Add (Variables|Default|GetBones) _returnvalue_2)))))

(fn ConstructionScript)

(fn GiveColorDependingonIndex
  (params (Index :type Integer))
  (bind _returnvalue (Math|Random|RandomFloat))
  (bind _returnvalue_2 (Math|Random|RandomFloat))
  (bind _returnvalue_3 (Math|Random|RandomFloat))
  (bind _returnvalue_4 (Math|Vector|MakeVector _returnvalue_2 _returnvalue_3 _returnvalue))
  (if (Variables|Skeleton|GetSameColorForEverything)
    (if (Variables|Skeleton|GetColorInitialized)
      (return (Variables|Skeleton|GetSameColor))
      (else
        (bind _output_get (Variables|Skeleton|SetSameColor _returnvalue_4))
        (Variables|Skeleton|SetColorInitialized true)
        (return _output_get)))
    (else
      (return _returnvalue_4))))

(fn MoveNodeto
  (params (IndexNode :type Integer) (NewLocation :type Vector))
  (Transformation|SetWorldLocation (Variables|/Script/Engine.Actor|GetRootComponent (Utilities|Array|Get(acopy) (Variables|Default|GetNodes) IndexNode)) NewLocation false false))

(fn ShowNodes
  (params (ShouldShow :type Boolean) (ShouldCollide :type ECollisionEnabled%20Enum :default "NoCollision"))
  (if ShouldShow
    (for _array_element (Variables|Default|GetNodes)
      (Collision|SetCollisionEnabled (Actor|GetComponentbyClass _array_element "/Script/Engine.StaticMeshComponent") ShouldCollide)
      (Rendering|SetVisibility (Actor|GetComponentbyClass _array_element "/Script/Engine.StaticMeshComponent") ShouldShow false)
      (Variables|Default|SetIsNodesVisible ShouldShow))
    (else
      (for _array_element_2 (Variables|Default|GetNodes)
        (Collision|SetCollisionEnabled (Actor|GetComponentbyClass _array_element_2 "/Script/Engine.StaticMeshComponent") ShouldCollide)
        (Rendering|SetVisibility (Actor|GetComponentbyClass _array_element_2 "/Script/Engine.StaticMeshComponent") ShouldShow false)
        (Variables|Default|SetIsNodesVisible ShouldShow)))))

(fn MoveNodestoKeypoints
  (params (KeypointsLocations :type Array%20of%20Vectors))
  (Variables|Default|SetKeypointsLocs KeypointsLocations)
  (for (_ _array_index) (Variables|Default|GetNodes)
    (CallFunction|MoveNodeto _array_index (+ (Utilities|Array|Get(acopy) (Variables|Default|GetKeypointsLocs) _array_index) "0.000000,-100.000000,0.000000"))))

(fn ShowBones
  (params (ShouldShow :type Boolean) (ShouldCollide :type ECollisionEnabled%20Enum :default "NoCollision"))
  (if ShouldShow
    (for _array_element (Variables|Default|GetBones)
      (Collision|SetCollisionEnabled (Actor|GetComponentbyClass _array_element "/Script/Engine.StaticMeshComponent") ShouldCollide)
      (Rendering|SetVisibility (Actor|GetComponentbyClass _array_element "/Script/Engine.StaticMeshComponent") ShouldShow false)
      (Variables|Default|SetIsBonesVisible ShouldShow))
    (else
      (for _array_element_2 (Variables|Default|GetBones)
        (Collision|SetCollisionEnabled (Actor|GetComponentbyClass _array_element_2 "/Script/Engine.StaticMeshComponent") ShouldCollide)
        (Rendering|SetVisibility (Actor|GetComponentbyClass _array_element_2 "/Script/Engine.StaticMeshComponent") ShouldShow false)
        (Variables|Default|SetIsBonesVisible ShouldShow)))))

(fn MoveBoneto
  (params (NewLoc1 :type Vector) (NewLoc2 :type Vector) (Index :type Integer))
  (Default|Moveto (Utilities|Array|Get(acopy) (Variables|Default|GetBones) Index) (+ NewLoc1 "0.000000,-100.000000,0.000000") (+ NewLoc2 "0.000000,-100.000000,0.000000")))

(fn MoveBonestoKeypoints
  (params (KeypointsLocations :type Array%20of%20Vectors))
  (bind _output_get (Variables|Default|SetKeypointsLocs KeypointsLocations))
  ;[1 1 1] Check Pose38
  (if (== (Utilities|Array|Length _output_get) 38)
    (for (_array_element _array_index) (Class|ZEDFunctionLibrary|GetBody38Bones)
      (CallFunction|MoveBoneto (Utilities|Array|Get(acopy) (Variables|Default|GetKeypointsLocs) (Math|Conversions|ToInteger(Byte) (.FirstEnd (Utilities|Struct|BreakSlBody38Bone _array_element)))) (Utilities|Array|Get(acopy) (Variables|Default|GetKeypointsLocs) (Math|Conversions|ToInteger(Byte) (.SecondEnd (Utilities|Struct|BreakSlBody38Bone _array_element)))) _array_index))
    (elif (== (Utilities|Array|Length _output_get) 70)
      (for (_array_element_2 _array_index_2) (Class|ZEDFunctionLibrary|GetBody70Bones)
        (CallFunction|MoveBoneto (Utilities|Array|Get(acopy) (Variables|Default|GetKeypointsLocs) (Math|Conversions|ToInteger(Byte) (.FirstEnd (Utilities|Struct|BreakSlBody70Bone _array_element_2)))) (Utilities|Array|Get(acopy) (Variables|Default|GetKeypointsLocs) (Math|Conversions|ToInteger(Byte) (.SecondEnd (Utilities|Struct|BreakSlBody70Bone _array_element_2)))) _array_index_2))
      (elif (== (Utilities|Array|Length _output_get) 34)
        (for (_array_element_3 _array_index_3) (Class|ZEDFunctionLibrary|GetBody34Bones)
          (CallFunction|MoveBoneto (Utilities|Array|Get(acopy) (Variables|Default|GetKeypointsLocs) (Math|Conversions|ToInteger(Byte) (.FirstEnd (Utilities|Struct|BreakSlBody34Bone _array_element_3)))) (Utilities|Array|Get(acopy) (Variables|Default|GetKeypointsLocs) (Math|Conversions|ToInteger(Byte) (.SecondEnd (Utilities|Struct|BreakSlBody34Bone _array_element_3)))) _array_index_3))))))