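; Body tracking visualizer that spawns and animates an avatar for each person the ZED camera detects.
; Optionally starts tracking when the camera is ready and adds a virtual canvas for the ZED image.
; On each new bodies frame, spawns or updates avatars keyed by body ID, feeding body data and smoothing, IK and height settings to ABP_ZED_Manny.
; Avatars of undetected IDs are destroyed; visibility can be toggled for all.
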(event Custom|Enable%20Body%20Tracking
  ;[1 1 1] Create Enable/Disable OD button in Editor
  (Class|ZEDCamera|EnableBodyTracking (Class|ZEDFunctionLibrary|GetCameraActor)))

(event Custom|Disable%20Body%20Tracking
  ;[1 1 1] Create Enable/Disable OD button in Editor
  (Class|ZEDCamera|DisableBodyTracking (Class|ZEDFunctionLibrary|GetCameraActor)))

(event Custom|ToggleAvatarVisibility
  (params (Visibility :type Boolean))
  ;[0 0.2871 1] toggle visibility
  (Variables|Default|SetAvatarsVisible Visibility)
  (Development|PrintString (Utilities|String|Append "Avatar ToggleVisibility [" (Utilities|String|ToString(Boolean) Visibility) "]"))
  (bind _values (Utilities|Map|Values (Variables|Default|GetAvatars)))
  (for _array_element _values
    (Rendering|SetVisibility (Actor|GetComponentbyClass _array_element "/Script/Engine.SkeletalMeshComponent") Visibility false)))

(event Custom|CustomEvent_1
  (params (bSuccess :type Boolean) (ErrorCode :type ESlErrorCode%20Enum :default "EC_Success") (Location :type Vector%20%28by%20ref%29) (Rotation :type Rotator%20%28by%20ref%29))
  ;[1 1 1] Enable OD automaticcly when the camera is ready (when tracking is enabled)
  (if (Variables|ZED|GetStartBodyTrackingAutomatically)
    (Class|ZEDCamera|EnableBodyTracking (Class|ZEDFunctionLibrary|GetCameraActor))))

(event Custom|OnRetrieveBodies
  (params (bodies :type Sl%20Bodies%20Structure%20%28by%20ref%29))
  (bind (_timestamp _bodylist _bisnew) (Utilities|Struct|BreakSlBodies bodies))
  ;[1 1 1] Bind event to retrieve object function
  (if _bisnew
    ;[1 1 1] Fill up the RemaningAvatars array.
    ; Used to know which person is no longer detected in the scene and destroy its avatar
    (bind _keys (Utilities|Map|Keys (Variables|Default|GetAvatars)))
    (Variables|Default|SetRemaining%20Avatars _keys)
    (for _array_element _bodylist
      (Variables|Default|SetCurrent%20Body _array_element)
      (Variables|Default|SetId (.Id (Utilities|Struct|BreakSlBodyData _array_element)))
      ;[1 1 1] If Tracking State is OK
      (if (Utilities|Enum|Equal(Enum) (.TrackingState (Utilities|Struct|BreakSlBodyData _array_element)) "OTS_Ok")
        (if (Utilities|Map|Contains (Variables|Default|GetAvatars) (.Id (Utilities|Struct|BreakSlBodyData _array_element)))
          (Utilities|Array|RemoveItem (Variables|Default|GetRemaining%20Avatars) (Variables|Default|GetId))
          ;[1 1 1] If the Avatar is already in the scene, only update its Skeletal Mesh
          (bind _output_get (Variables|Default|SetSkeletal%20Mesh (Actor|GetComponentbyClass (.Value (Utilities|Map|Find (Variables|Default|GetAvatars) (Variables|Default|GetId))) "/Script/Engine.SkeletalMeshComponent")))
          (Variables|/Game/ZED/Blueprints/BodyTracking/ABP_ZED_Manny.ABP_ZED_Manny_C|SetBody%20%20Data (.AsABP%20ZED%20Manny (Utilities|Casting|CastToABP_ZED_Manny (Components|SkeletalMesh|GetAnimInstance _output_get))) (Variables|Default|GetCurrent%20Body))
          (Variables|/Game/ZED/Blueprints/BodyTracking/ABP_ZED_Manny.ABP_ZED_Manny_C|SetEnableFootIK (.AsABP%20ZED%20Manny (Utilities|Casting|CastToABP_ZED_Manny (Components|SkeletalMesh|GetAnimInstance _output_get))) (Variables|AnimParameters|GetEnableFootIK))
          (Variables|/Game/ZED/Blueprints/BodyTracking/ABP_ZED_Manny.ABP_ZED_Manny_C|SetHeight%20Offset (.AsABP%20ZED%20Manny (Utilities|Casting|CastToABP_ZED_Manny (Components|SkeletalMesh|GetAnimInstance _output_get))) (Variables|AnimParameters|GetHeight%20Offset))
          (CallFunction|UpdateSmoothingParams (.AsABP%20ZED%20Manny (Utilities|Casting|CastToABP_ZED_Manny (Components|SkeletalMesh|GetAnimInstance _output_get))))
          (else
            ;[1 1 1] New Detection : Spawn a new Avatar and update its Skeletal Mesh with Body Tracking Data
            (bind _returnvalue (Game|SpawnActorfromClass (Variables|ZED|GetActor%20Class) (Variables|Default|GetSpawn%20Transform) "Undefined" 0 0))
            (Utilities|Map|Add (Variables|Default|GetAvatars) (Variables|Default|GetId) _returnvalue)
            (Variables|Default|SetSkeletal%20Mesh (Actor|GetComponentbyClass _returnvalue "/Script/Engine.SkeletalMeshComponent"))
            (Rendering|SetVisibility (Actor|GetComponentbyClass _returnvalue "/Script/Engine.SkeletalMeshComponent") (Variables|Default|GetAvatarsVisible) false)
            (bind _asbp_zed_manny (Utilities|Casting|CastToBP_ZED_Manny _returnvalue))
            (if (Variables|AnimParameters|GetEnableSelfCollision)
              (Default|EnableSelfCollision _asbp_zed_manny))
            (Variables|/Game/ZED/Blueprints/BodyTracking/ABP_ZED_Manny.ABP_ZED_Manny_C|SetBody%20%20Data (.AsABP%20ZED%20Manny (Utilities|Casting|CastToABP_ZED_Manny (Components|SkeletalMesh|GetAnimInstance (Actor|GetComponentbyClass _returnvalue "/Script/Engine.SkeletalMeshComponent")))) (Variables|Default|GetCurrent%20Body))
            (Variables|/Game/ZED/Blueprints/BodyTracking/ABP_ZED_Manny.ABP_ZED_Manny_C|SetSkeletal%20Mesh (.AsABP%20ZED%20Manny (Utilities|Casting|CastToABP_ZED_Manny (Components|SkeletalMesh|GetAnimInstance (Actor|GetComponentbyClass _returnvalue "/Script/Engine.SkeletalMeshComponent")))) (Variables|Default|GetSkeletal%20Mesh))
            (Variables|/Game/ZED/Blueprints/BodyTracking/ABP_ZED_Manny.ABP_ZED_Manny_C|SetBoneScaling (.AsABP%20ZED%20Manny (Utilities|Casting|CastToABP_ZED_Manny (Components|SkeletalMesh|GetAnimInstance (Actor|GetComponentbyClass _returnvalue "/Script/Engine.SkeletalMeshComponent")))) (Variables|AnimParameters|GetBone%20Scaling%20-%20Experimental))
            (Variables|/Game/ZED/Blueprints/BodyTracking/ABP_ZED_Manny.ABP_ZED_Manny_C|SetHeight%20Offset (.AsABP%20ZED%20Manny (Utilities|Casting|CastToABP_ZED_Manny (Components|SkeletalMesh|GetAnimInstance (Actor|GetComponentbyClass _returnvalue "/Script/Engine.SkeletalMeshComponent")))) (Variables|AnimParameters|GetHeight%20Offset))
            (Variables|/Game/ZED/Blueprints/BodyTracking/ABP_ZED_Manny.ABP_ZED_Manny_C|SetStick%20Avatar%20On%20Floor (.AsABP%20ZED%20Manny (Utilities|Casting|CastToABP_ZED_Manny (Components|SkeletalMesh|GetAnimInstance (Actor|GetComponentbyClass _returnvalue "/Script/Engine.SkeletalMeshComponent")))) (Variables|AnimParameters|GetStick%20Avatar%20on%20Floor))
            (Variables|/Game/ZED/Blueprints/BodyTracking/ABP_ZED_Manny.ABP_ZED_Manny_C|SetEnableFootIK (.AsABP%20ZED%20Manny (Utilities|Casting|CastToABP_ZED_Manny (Components|SkeletalMesh|GetAnimInstance (Actor|GetComponentbyClass _returnvalue "/Script/Engine.SkeletalMeshComponent")))) (Variables|AnimParameters|GetEnableFootIK))
            (CallFunction|UpdateSmoothingParams (.AsABP%20ZED%20Manny (Utilities|Casting|CastToABP_ZED_Manny (Components|SkeletalMesh|GetAnimInstance (Actor|GetComponentbyClass _returnvalue "/Script/Engine.SkeletalMeshComponent")))))))))
    ;[1 1 1] Destroy Avatars which are not longer detected in the scene
    (for _array_element_2 (Variables|Default|GetRemaining%20Avatars)
      (if (== (.ReturnValue (Utilities|Map|Find (Variables|Default|GetAvatars) _array_element_2)) true)
        (Actor|DestroyActor (.Value (Utilities|Map|Find (Variables|Default|GetAvatars) _array_element_2)))
        (Utilities|Map|Remove (Variables|Default|GetAvatars) _array_element_2)))))

(event EventBeginPlay
  (Utilities|FlowControl|Sequence
    (:then_0
      ;[1 1 1] Enable OD automaticcly when the camera is ready (when tracking is enabled)
      (EventDispatchers|AssignOnTrackingEnabled (Class|SlFunctionLibrary|GetCameraProxy) (delegate Custom|CustomEvent_1)))
    (:then_1
      ;[1 1 1] Create canvas to display ZED Image on the screen
      (bind _returnvalue (UserInterface|CreateWidget "/Game/ZED/Blueprints/BodyTracking/BP_VirtualCanvas.BP_VirtualCanvas_C"))
      (UserInterface|Viewport|AddtoViewport _returnvalue 0))
    (:then_2
      ;[1 1 1] Bind event to retrieve object function
      (EventDispatchers|BindEventtoOnBodyTrackingRetrieved (Class|SlFunctionLibrary|GetCameraProxy) (delegate Custom|OnRetrieveBodies)))))

(fn ConstructionScript)

(fn UpdateSmoothingParams
  (params (ABP_ZED_Manny :type ABP%20ZED%20Manny%20Object%20Reference))
  (Variables|/Game/ZED/Blueprints/BodyTracking/ABP_ZED_Manny.ABP_ZED_Manny_C|SetRotation%20Slerp%20Intensity ABP_ZED_Manny (Variables|AnimParameters|GetJointRotationSmoothing))
  (Variables|/Game/ZED/Blueprints/BodyTracking/ABP_ZED_Manny.ABP_ZED_Manny_C|SetRoot%20Location%20Slerp%20Intensity ABP_ZED_Manny (Variables|AnimParameters|GetRootTranslationSmoothing)))