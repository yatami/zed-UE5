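; Visualizer actor that shows ZED camera object detections as 3D bounding boxes in the scene.
; It binds to camera proxy events, optionally enabling detection once tracking starts, and exposes enable and disable events.
; Each retrieved detection set updates a map of BP_BBox3D actors keyed by object ID, spawning boxes for new IDs.
; A copy of the map keys, pruned as objects match, identifies stale boxes to destroy.
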(event Custom|Disable%20OD
  ;[1 1 1] Create Enable/Disable OD button in Editor
  (Class|ZEDCamera|DisableObjectDetection (Class|ZEDFunctionLibrary|GetCameraActor)))

(event Custom|Enable%20OD
  ;[1 1 1] Create Enable/Disable OD button in Editor
  (Class|ZEDCamera|EnableObjectDetection (Class|ZEDFunctionLibrary|GetCameraActor)))

(event Custom|OnObjectDetectionRetrieved_Event_1
  (params (objects :type Sl%20Objects%20Structure%20%28by%20ref%29))
  ;[1 1 1] Bind event to retrieve object function
  ;[1 1 1] Fill up the ActiveID array.
  ; Used to know which person is no longer detected in the scene and destroy its box
  (bind _keys (Utilities|Map|Keys (Variables|Default|Get3D%20Boxes)))
  (Variables|Default|SetActive%20IDs _keys)
  (for _array_element (.ObjectList (Utilities|Struct|BreakSlObjects objects))
    (bind _output_get (Variables|Default|SetCurrent%20ObjectData _array_element))
    (bind _output_get_2 (Variables|Default|SetId (.Id (Utilities|Struct|BreakSlObjectData _output_get))))
    ;[1 1 1] If the Box is already in the scene, only update its Transform
    (if (Utilities|Map|Contains (Variables|Default|Get3D%20Boxes) _output_get_2)
      (Utilities|Array|RemoveItem (Variables|Default|GetActive%20IDs) (Variables|Default|GetId))
      (Class|SlFunctionLibrary|Set3DBoxTransform (.Value (Utilities|Map|Find (Variables|Default|Get3D%20Boxes) (Variables|Default|GetId))) (Variables|Default|GetCurrent%20ObjectData))
      (else
        ;[1 1 1] New Detection : Spawn a new Box and update its position, rotation and scale
        (bind _returnvalue (Game|SpawnActorfromClass "/Game/ZED/Blueprints/ObjectDetection/BP_BBox3D.BP_BBox3D_C" (Variables|Default|GetTransform) "Undefined" 0 0))
        (Utilities|Map|Add (Variables|Default|Get3D%20Boxes) (Variables|Default|GetId) _returnvalue)
        (Class|SlFunctionLibrary|Set3DBoxTransform _returnvalue (Variables|Default|GetCurrent%20ObjectData)))))
  ;[1 1 1] Destroy Boxes which are not longer detected in the scene
  (for _array_element_2 (Variables|Default|GetActive%20IDs)
    (if (== (.ReturnValue (Utilities|Map|Find (Variables|Default|Get3D%20Boxes) _array_element_2)) true)
      (Actor|DestroyActor (.Value (Utilities|Map|Find (Variables|Default|Get3D%20Boxes) _array_element_2)))
      (Utilities|Map|Remove (Variables|Default|Get3D%20Boxes) _array_element_2))))

(event Custom|OnTrackingEnabled_Event_0
  (params (bSuccess :type Boolean) (ErrorCode :type ESlErrorCode%20Enum :default "EC_Success") (Location :type Vector%20%28by%20ref%29) (Rotation :type Rotator%20%28by%20ref%29))
  ;[1 1 1] Enable OD automaticcly when the camera is ready (when tracking is enabled)
  (if (Variables|ZED|GetStart%20Object%20Detection%20Automatically)
    (Class|ZEDCamera|EnableObjectDetection (Class|ZEDFunctionLibrary|GetCameraActor))))

(event EventBeginPlay
  (Utilities|FlowControl|Sequence
    (:then_1
      ;[1 1 1] Bind event to retrieve object function
      (EventDispatchers|AssignOnObjectDetectionRetrieved (Class|SlFunctionLibrary|GetCameraProxy) (delegate Custom|OnObjectDetectionRetrieved_Event_1)))
    (:then_2
      ;[1 1 1] Enable OD automaticcly when the camera is ready (when tracking is enabled)
      (EventDispatchers|AssignOnTrackingEnabled (Class|SlFunctionLibrary|GetCameraProxy) (delegate Custom|OnTrackingEnabled_Event_0)))))

(fn ConstructionScript)